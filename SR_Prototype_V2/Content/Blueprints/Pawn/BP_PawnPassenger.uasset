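; Passenger pawn that walks a looping route of movement points across decks and heads for a muster station during an emergency.
; SearchForClosestMovementPoint takes the next point by index, not distance, routing via the current floor's staircase when the target deck differs.
; On same-deck moves, a timer teleports the pawn to its point if not cancelled by OverlappedOnePoint.
; The Emergency event toggles muster mode, resuming the route immediately only when switched off.
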(event `SearchForClosestMovementPoint`
  (bind _pawncontrollerref (`self.PawnControllerRef`))
  (bind _currentfloor (`self.CurrentFloor`))
  (bind _output (`|GetArrayItem` (`self.MovementPointsArray`) (`self.IndexToWalkTo`)))
  (bind _deckref (`/Game/Blueprints/Pawn/BP_MovementPoints.DeckRef` _output))
  ;[1 1 1] Get the pawn to move to the next point
  (if (`self.Emergency?`)
    (for _array_element (`self.Floors`)
      (if (`/Game/Blueprints/Ship/BP_Floor.HasMuster?` _array_element)
        (bind _output_get (set `self.FloorToMoveTo` _array_element))
        (set `self.OnFloor?` (== _output_get _currentfloor))))
    (if (`self.OnFloor?`)
      (`NavigationSystem.SimpleMoveToLocation` _pawncontrollerref (`SceneComponent.K2_GetComponentLocation` (`/Game/Blueprints/Ship/BP_Floor.MusterStation` _currentfloor)))
      (else
        (`/Engine/EditorBlueprintResources/StandardMacros.DoOnce` false :!label _label
          (:`Completed`
            (`NavigationSystem.SimpleMoveToLocation` _pawncontrollerref (`SceneComponent.K2_GetComponentLocation` (`/Game/Blueprints/Ship/BP_Floor.StaircaseBox` _currentfloor)))))))
    (elif (not (== (`self.CurrentFloor`) _deckref))
      (set `self.FloorToMoveTo` _deckref)
      (`NavigationSystem.SimpleMoveToLocation` (`self.PawnControllerRef`) (`SceneComponent.K2_GetComponentLocation` (`/Game/Blueprints/Ship/BP_Floor.StaircaseBox` (`self.CurrentFloor`))))
      (else
        (`NavigationSystem.SimpleMoveToActor` (`self.PawnControllerRef`) _output)
        (bind _returnvalue (`KismetSystemLibrary.K2_SetTimerDelegate` (delegate `Resetposition`) 3.0))
        (set `self.ResetHandle` _returnvalue)))))

(event `Reset`
  ;[1 1 1] Get the pawn to move to the next point
  (goto _label :!via `Reset`))

(event `Resetposition`
  ;[1 1 1] Get the pawn to move to the next point
  (`self.K2_SetActorLocation` (`self.K2_GetActorLocation` (`|GetArrayItem` (`self.MovementPointsArray`) (`self.IndexToWalkTo`))))
  (`self.OverlappedOnePoint`))

(event `Emergency`
  (if (`self.Emergency?`)
    (set `self.Emergency?` false)
    (`self.SearchForClosestMovementPoint`)
    (else
      (set `self.Emergency?` true))))

(event `self.ReceiveBeginPlay`
  (`parent.ReceiveBeginPlay`))

(event `MoveToMuster`
  ;[1 1 1] USE FOR GO TO MUSTER
  (if (`self.Emergency?`)
    (`NavigationSystem.SimpleMoveToLocation` (`self.PawnControllerRef`) (`SceneComponent.K2_GetComponentLocation` (`/Game/Blueprints/Ship/BP_Floor.MusterStation` (`self.FloorToMoveTo`))))
    (else
      (`self.SearchForClosestMovementPoint`))))

(event `OverlappedOnePoint`
  ;[1 1 1] Call This when the pawn Overlaps a movement point, then make the pawn find a new point to walk to.
  (`KismetSystemLibrary.K2_ClearAndInvalidateTimerHandle` (`self.ResetHandle`))
  (bind _output_get (set `self.IndexToWalkTo` (+ (`self.IndexToWalkTo`) 1)))
  (if (> _output_get (- (`KismetArrayLibrary.Array_Length` (`self.MovementPointsArray`)) 1))
    (set `self.IndexToWalkTo` 0)
    (`self.SearchForClosestMovementPoint`)
    (else
      (`self.SearchForClosestMovementPoint`))))

(fn `UserConstructionScript`
  (`parent.UserConstructionScript`))