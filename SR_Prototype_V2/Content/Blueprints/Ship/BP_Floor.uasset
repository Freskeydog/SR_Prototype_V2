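; BP_Floor is a single deck floor of a ship that shows its deck image and name and can be clicked.
; SetValuesToFloor applies the deck image through a dynamic M_Deck material, sets the name text and stores the deck index.
; On BeginPlay it fades the trigger mesh to low opacity and caches its location.
; Clicking the trigger mesh passes itself and that location to the ship Blueprint's FloorClicked.
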(event `self.ReceiveBeginPlay`
  (`MeshComponent.SetScalarParameterValueOnMaterials` (`self.TriggerMesh`) "Opacity" 0.2)
  (bind _output_get (set `self.FloorLocation` (`self.K2_GetActorLocation`)))
  (`KismetSystemLibrary.PrintString` (`KismetStringLibrary.Conv_VectorToString` _output_get)))

(event `self.TriggerMesh.OnClicked`
  (params (TouchedComponent :type "PrimitiveComponent Object Reference") (ButtonPressed :type "Key Structure" :default "AnyKey"))
  (`KismetSystemLibrary.PrintString` (`KismetSystemLibrary.GetDisplayName` TouchedComponent))
  (`/Game/Blueprints/Ship/BP_Ship.FloorClicked` (`self.BP_ShipRef`) self (`self.FloorLocation`)))

(fn `SetValuesToFloor`
  (params (DeckImage :type "Texture Object Reference") (DeckName :type Text) (DeckIndex :type Integer))
  (bind _returnvalue (`PrimitiveComponent.CreateDynamicMaterialInstance` (`self.Floor_Mesh`) 0 "/Game/Materials/M_Deck.M_Deck"))
  (set `self.Material` _returnvalue)
  (`TextRenderComponent.K2_SetText` (`self.TextRender`) DeckName)
  (`MaterialInstanceDynamic.SetTextureParameterValue` (`self.Material`) "DeckImage" DeckImage)
  (set `self.FloorIndex` DeckIndex)
  (return))

(fn `UserConstructionScript`)