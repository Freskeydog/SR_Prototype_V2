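; Ship actor that displays its decks as BP_Floor actors in a switchable list or grid view, navigated with an orthographic camera.
; Construction script previews decks as child actors, which BeginPlay replaces with spawned floors before creating the main widget.
; A recursive function lays out grid rows, and cached positions drive view switching.
; Variable-length timelines animate scrolling, click-to-deck moves and zoom, with flags gating overlapping input.
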(event `AddRealDeckActors`
  (bind _decks (`self.Decks`))
  (bind _deckstartingpos (`self.DeckStartingPos`))
  (bind ((`DistanceBetweenFloors_7_4ECEC1AA4DF2B8434F59AABE5F8F5FCA` _distancebetweenfloors) (`NameSize_9_7556AA284F455C187F2E3E85FC87BF16` _namesize) (`TriggerScale_22_EF520A1244B90B5CD1394D9B2D0A12F0` _triggerscale) (`DeckScale_21_88CECE8E4A64988FBC393A8AF6C8430C` _deckscale) (`NameLocation_18_07272B6744170C076B9F83B48BC6B58E` _namelocation)) (break `/Game/Blueprints/Structs/s_DeckSetup` (`self.DeckListSetup`)))
  ;[1 1 1] Deletes construction script child actors and creates actors of same BP to replace with same values.
  (for _array_element _decks
    (`self.K2_DestroyActor` _array_element))
  (`KismetArrayLibrary.Array_Clear` _decks)
  (for (_array_element_2 _array_index) (`self.GetFloors`)
    (bind (_floorname _floorimage) (break `/Game/Blueprints/Structs/s_FloorInfo` _array_element_2))
    (bind _returnvalue (`|SpawnActorFromClass` "/Game/Blueprints/Ship/BP_Floor.BP_Floor_C" (`KismetMathLibrary.MakeTransform` _deckstartingpos (struct) (`KismetMathLibrary.MakeVector` _deckscale _deckscale _deckscale)) "Undefined" "OverrideRootScale" null _floorname _array_index _floorimage self))
    (`self.f_CreateNewDecksForGameplay` _floorname _floorimage _array_index _namesize _triggerscale _namelocation _returnvalue)
    (set `/Game/Blueprints/Ship/BP_Floor.FloorListLocation` _deckstartingpos _returnvalue)
    (set `self.DeckStartingPos` (+ _deckstartingpos (`KismetMathLibrary.MakeVector` 0.0 _distancebetweenfloors))))
  (for _array_element_3 (`self.Decks`)
    (`KismetArrayLibrary.Array_Add` (`self.DeckListPositions`) (`/Game/Blueprints/Ship/BP_Floor.FloorListLocation` _array_element_3)))
  (`self.CreateGridSetup`)
  (bind _returnvalue_2 (`|CreateWidget` "/Game/Blueprints/Widgets/w_Main.w_Main_C"))
  (bind _output_get (set `self.MainWidget` _returnvalue_2))
  (set `/Game/Blueprints/Widgets/w_Main.ShipRef` self _output_get)
  (`UserWidget.AddToViewport` _output_get 0))

(event `ScrollUp`
  (bind (_maxscrollup _nextvalue _truefalse) (`self.f_SmoothScrollUp`))
  ;[1 1 1] Scroll up and down functions with smooth scroll
  (if (`self.f_CanScroll?`)
    (if (`self.SmoothScroll?`)
      (`TimelineComponent.SetTimelineLength` (`self.SmoothScrollUp`) (`self.SmoothScrollTime`))
      (set `self.CanScroll?` false)
      (set `self.ScrollTo` (select `bool` _truefalse :`false` _nextvalue :`true` _maxscrollup))
      (`Timeline|SmoothScrollUp` :!via `PlayFromStart`
        (:`Update`
          (`self.K2_SetActorLocation` (`self.CameraRef`) (`KismetMathLibrary.VLerp` (`self.GetCameraLocation`) (`self.ScrollTo`) (`self.GetAlphaForTimeline` (`self.SmoothScrollUp`))) false false))
        (:`Finished`
          (set `self.CanScroll?` true)))
      (else
        (`self.f_ScrollUp`)))))

(event `ScrollDown`
  (bind (_true _false _truefalse) (`self.f_SmoothScrollDown`))
  ;[1 1 1] Scroll up and down functions with smooth scroll
  (if (`self.f_CanScroll?`)
    (if (`self.SmoothScroll?`)
      (`TimelineComponent.SetTimelineLength` (`self.SmoothScrollDown`) (`self.SmoothScrollTime`))
      (set `self.CanScroll?` false)
      (set `self.ScrollTo` (select `bool` _truefalse :`false` _false :`true` _true))
      (`Timeline|SmoothScrollDown` :!via `PlayFromStart`
        (:`Update`
          (`self.K2_SetActorLocation` (`self.CameraRef`) (`KismetMathLibrary.VLerp` (`self.GetCameraLocation`) (`self.ScrollTo`) (`self.GetAlphaForTimeline` (`self.SmoothScrollDown`))) false false))
        (:`Finished`
          (set `self.CanScroll?` true)))
      (else
        (`self.f_ScrollDown`)))))

(event `CreateGridSetup`
  (bind _decks (`self.Decks`))
  ;[1 1 1] Deletes construction script child actors and creates actors of same BP to replace with same values.
  (`KismetSystemLibrary.Delay` 0.3)
  (`self.GenerateGridPattern` _decks)
  (set `self.PreviouslySelectedDeck` (`|GetArrayItem` _decks)))

(event `self.ReceiveBeginPlay`
  (bind (_controller _bsuccess) (`self.GetController`))
  ;[1 1 1] Creates references and Creates deck actors
  (if _bsuccess
    (`/Game/Blueprints/Ruleset/ScanReach_Con.AddShipRef` _controller self)
    (`self.f_GetScrollDownInfo`)
    (`CameraComponent.SetOrthoWidth` (`CameraActor.CameraComponent` (`self.CameraRef`)) (`self.CamereDefaultValue`))
    (`self.AddRealDeckActors`)
    (set `self.CameraDefaultLocation` (`self.GetCameraLocation`))))

(event `CreateCameraRef`
  (params (Camera :type "CameraActor Object Reference"))
  ;[1 1 1] Creates references and Creates deck actors
  (set `self.CameraRef` Camera))

(event `ChangeListToGrid`
  (bind _cameraref (`self.CameraRef`))
  (bind _previouslyselecteddeck (`self.PreviouslySelectedDeck`))
  ;[1 1 1] Change from list view to grid view and reverse
  (if (not (`self.DeckGrid?`))
    (for (_array_element _array_index) (`self.Decks`)
      (`self.K2_SetActorLocation` _array_element (`|GetArrayItem` (`self.DeckGridPositions`) _array_index) false false)
      (set `self.DeckGrid?` true)
      (`CameraComponent.SetOrthoWidth` (`CameraActor.CameraComponent` _cameraref) (select `bool` (`self.DeckGrid?`) :`false` (`self.CamereDefaultValue`) :`true` (`self.CameraGridValue`)) :!label _label)
      (`/Engine/EditorBlueprintResources/StandardMacros.IsValid` _previouslyselecteddeck
        (:`Is Valid`
          (`self.K2_SetActorLocation` _cameraref (select `bool` (`self.DeckGrid?`) :`false` (`KismetMathLibrary.MakeVector` (.x (`self.CameraDefaultLocation`)) (.y (`/Game/Blueprints/Ship/BP_Floor.FloorListLocation` _previouslyselecteddeck)) 500.0) :`true` (`KismetMathLibrary.MakeVector` 2000.0 (* (`.DistanceBetweenFloors_7_4ECEC1AA4DF2B8434F59AABE5F8F5FCA` (break `/Game/Blueprints/Structs/s_DeckSetup` (`self.DeckListSetup`))) 2.0) 500.0)) false false))
        (:`Is Not Valid`
          (`self.K2_SetActorLocation` (select `bool` (`self.DeckGrid?`) :`false` (`self.CameraDefaultLocation`) :`true` (`self.CameraDefaultGridLocation`))))))
    (else
      (for (_array_element_2 _array_index_2) (`self.Decks`)
        (`self.K2_SetActorLocation` _array_element_2 (`|GetArrayItem` (`self.DeckListPositions`) _array_index_2) false false)
        (set `self.DeckGrid?` false)
        (goto _label)))))

(event `FloorClicked`
  (params (Floor :type "/Game/Blueprints/Ship/BP_Floor Object Reference") (FloorLocation :type "Vector Structure"))
  ;[1 1 1] move camera to chosen floor
  (if (`self.CanClick?`)
    (if (not (== Floor (`self.SelectedDeck`)))
      (set `self.CanClick?` false)
      (set `self.SelectedDeck` Floor)
      (bind _cameratogoto (`self.f_FindCameraScrollDownLocation` FloorLocation Floor))
      (`TimelineComponent.SetTimelineLength` (`self.ClickedScroll`) (select `bool` (`self.WasOverviewButton?`) :`false` (`self.ClickedScrollTime`) :`true` (`self.ClickedScrollTimeButton`)))
      (set `self.CanScroll?` false)
      (`Timeline|ClickedScroll` :!via `PlayFromStart`
        (:`Update`
          (`self.K2_SetActorLocation` (`self.CameraRef`) (`KismetMathLibrary.VLerp` (`self.GetCameraLocation`) _cameratogoto (`self.GetAlphaForTimeline` (`self.ClickedScroll`))) false false))
        (:`Finished`
          (set `self.WasOverviewButton?` false)
          (set `self.CanScroll?` true)
          (set `self.CanClick?` true)
          (set `self.PreviouslySelectedDeck` (`self.SelectedDeck`))
          (set `self.SelectedDeck` null))))))

(event `StartClickedZoom`
  (bind _cameraref (`self.CameraRef`))
  (bind _alpha (`self.GetAlphaForTimeline` (`self.ClickedZoom`)))
  ;[1 1 1] Zoom in to clicked deck if clicked in viewport. Check if autozoom is enabled if clicked in deck overview
  (`TimelineComponent.SetTimelineLength` (`self.ClickedZoom`) (`self.ClickedZoomTime`))
  (set `self.ClickZoomReverse?` false)
  (set `self.IsZoomed?` true)
  (set `self.CameraDefaultLocation` (`self.GetCameraLocation`))
  (set `self.CameraToZoomLocation` (`KismetMathLibrary.MakeVector` 0.0 (.y (`self.GetCameraLocation`)) (.z (`self.GetCameraLocation`))))
  (`Timeline|ClickedZoom` :!via `PlayFromStart` :!label _label_2
    (:`Update`
      (`CameraComponent.SetOrthoWidth` (`CameraActor.CameraComponent` _cameraref) (`KismetMathLibrary.Lerp` (`self.CamereDefaultValue`) (`self.CameraZoomValue`) _alpha))
      (`self.K2_SetActorLocation` _cameraref (`KismetMathLibrary.VLerp` (`self.CameraDefaultLocation`) (`self.CameraToZoomLocation`) _alpha) false false))
    (:`Finished`
      (set `self.CanClick?` true)
      (if (`self.ClickZoomReverse?`)
        _))))

(event `ReverseZoom`
  ;[1 1 1] Zoom in to clicked deck if clicked in viewport. Check if autozoom is enabled if clicked in deck overview
  (`TimelineComponent.SetTimelineLength` (`self.ClickedZoom`) (`self.ClickedZoomTime`))
  (set `self.ClickZoomReverse?` true)
  (goto _label_2 :!via `ReverseFromEnd`))

(fn `f_CanScroll?`
  (returns (`CanScroll?` :type Boolean))
  (return (and (`self.CanScroll?`) (not (`self.IsZoomed?`)))))

(fn `f_CreateNewDeck`
  (params (`Deck Name` :type Text) (`Deck Image` :type "Texture Object Reference") (`Deck Index` :type Integer) (`Deck Location` :type "Vector Structure") (DeckScale :type "Float (double-precision)") (NameSize :type "Float (double-precision)") (TriggerScale :type "Vector Structure") (NameLocation :type "Vector Structure"))
  (bind _returnvalue (`AddComponent|NODE_AddChildActorComponent-1` :`RelativeTransform` (`KismetMathLibrary.MakeTransform` `Deck Location` (struct) (`KismetMathLibrary.MakeVector` DeckScale DeckScale DeckScale))))
  (bind _asbp_floor (cast `/Game/Blueprints/Ship/BP_Floor` (`ChildActorComponent.ChildActor` _returnvalue)))
  (set `/Game/Blueprints/Ship/BP_Floor.BP_ShipRef` self _asbp_floor)
  (`KismetArrayLibrary.Array_AddUnique` (`self.Decks`) _asbp_floor)
  (`SceneComponent.SetWorldScale3D` (`/Game/Blueprints/Ship/BP_Floor.TriggerMesh` _asbp_floor) TriggerScale)
  (`TextRenderComponent.SetWorldSize` (`/Game/Blueprints/Ship/BP_Floor.TextRender` _asbp_floor) NameSize)
  (`SceneComponent.K2_AddWorldOffset` (`/Game/Blueprints/Ship/BP_Floor.TextRender` _asbp_floor) NameLocation false false)
  (`/Game/Blueprints/Ship/BP_Floor.SetValuesToFloor` _asbp_floor `Deck Image` `Deck Name` `Deck Index`)
  (return))

(fn `f_CreateNewDecksForGameplay`
  (params (`Deck Name` :type Text) (`Deck Image` :type "Texture Object Reference") (`Deck Index` :type Integer) (NameSize :type "Float (double-precision)") (TriggerScale :type "Vector Structure") (NameLocation :type "Vector Structure") (Deck :type "/Game/Blueprints/Ship/BP_Floor Object Reference"))
  (set `/Game/Blueprints/Ship/BP_Floor.BP_ShipRef` self Deck)
  (`KismetArrayLibrary.Array_AddUnique` (`self.Decks`) Deck)
  (`SceneComponent.SetWorldScale3D` (`/Game/Blueprints/Ship/BP_Floor.TriggerMesh` Deck) TriggerScale)
  (`TextRenderComponent.SetWorldSize` (`/Game/Blueprints/Ship/BP_Floor.TextRender` Deck) NameSize)
  (`SceneComponent.K2_AddWorldOffset` (`/Game/Blueprints/Ship/BP_Floor.TextRender` Deck) NameLocation false false)
  (`/Game/Blueprints/Ship/BP_Floor.SetValuesToFloor` Deck `Deck Image` `Deck Name` `Deck Index`)
  (return))

(fn `f_FindCameraScrollDownLocation`
  (params (`Location Y` :type "Vector Structure") (ActorRef :type "Actor Object Reference"))
  (returns (CameraToGoTo :type "Vector Structure"))
  (`/Engine/EditorBlueprintResources/StandardMacros.IsValid` ActorRef
    (:`Is Valid`
      (return (`KismetMathLibrary.MakeVector` (.x (`self.GetCameraLocation`)) (.y `Location Y`) (.z (`self.GetCameraLocation`)))))))

(fn `f_GetScrollDownInfo`
  (bind _returnvalue_x (`KismetMathLibrary.BreakVector` (`self.K2_GetActorLocation`)))
  (bind _returnvalue_x_2 (`KismetMathLibrary.BreakVector` (`self.K2_GetActorLocation`)))
  (bind ((`Decks_15_4BEBB74B4BD5233113329891216757F0` _decks) (`DistanceBetweenFloors_7_4ECEC1AA4DF2B8434F59AABE5F8F5FCA` _distancebetweenfloors)) (break `/Game/Blueprints/Structs/s_DeckSetup` (`self.DeckListSetup`)))
  (bind _returnvalue (* (`KismetArrayLibrary.Array_LastIndex` _decks) _distancebetweenfloors))
  (set `self.MinScrollDownValue` _returnvalue)
  (set `self.MinScrollDownValueGrid` (/ _returnvalue 2.0))
  (set `self.MinScrollDownPos` (`KismetMathLibrary.MakeVector` _returnvalue_x (`self.MinScrollDownValue`) 500.0))
  (set `self.MinScrollDownPosGrid` (`KismetMathLibrary.MakeVector` _returnvalue_x_2 (`self.MinScrollDownValueGrid`) 500.0))
  (return))

(fn `f_ScrollDown`
  (if (<= (select `bool` (`self.DeckGrid?`) :`false` (`self.MinScrollDownValue`) :`true` (`self.MinScrollDownValueGrid`)) (.y (`self.GetCameraLocation`)))
    (`self.K2_SetActorLocation` (`self.CameraRef`) (`KismetMathLibrary.MakeVector` (.x (`self.GetCameraLocation`)) (select `bool` (`self.DeckGrid?`) :`false` (`self.MinScrollDownValue`) :`true` (`self.MinScrollDownValueGrid`)) (.z (`self.GetCameraLocation`))) false false)
    (else
      (`self.K2_SetActorLocation` (`self.CameraRef`) (`KismetMathLibrary.MakeVector` (.x (`self.GetCameraLocation`)) (+ (.y (`self.GetCameraLocation`)) (`.DistanceBetweenFloors_7_4ECEC1AA4DF2B8434F59AABE5F8F5FCA` (break `/Game/Blueprints/Structs/s_DeckSetup` (`self.DeckListSetup`)))) (.z (`self.GetCameraLocation`))) false false))))

(fn `f_ScrollUp`
  (if (<= (.y (`self.GetCameraLocation`)) (select `bool` (`self.DeckGrid?`) :`true` (* (`.DistanceBetweenFloors_7_4ECEC1AA4DF2B8434F59AABE5F8F5FCA` (break `/Game/Blueprints/Structs/s_DeckSetup` (`self.DeckListSetup`))) 2.0)))
    (`self.K2_SetActorLocation` (`self.CameraRef`) (`KismetMathLibrary.MakeVector` (.x (`self.GetCameraLocation`)) (select `bool` (`self.DeckGrid?`) :`true` (* (`.DistanceBetweenFloors_7_4ECEC1AA4DF2B8434F59AABE5F8F5FCA` (break `/Game/Blueprints/Structs/s_DeckSetup` (`self.DeckListSetup`))) 2.0)) (.z (`self.GetCameraLocation`))) false false)
    (else
      (`self.K2_SetActorLocation` (`self.CameraRef`) (`KismetMathLibrary.MakeVector` (.x (`self.GetCameraLocation`)) (- (.y (`self.GetCameraLocation`)) (`.DistanceBetweenFloors_7_4ECEC1AA4DF2B8434F59AABE5F8F5FCA` (break `/Game/Blueprints/Structs/s_DeckSetup` (`self.DeckListSetup`)))) (.z (`self.GetCameraLocation`))) false false))))

(fn `f_SmoothScrollDown`
  (returns (True :type "Vector Structure") (False :type "Vector Structure") (TrueFalse :type Boolean))
  (bind _returnvalue (`self.K2_GetActorLocation` (`self.CameraRef`)))
  (return (`KismetMathLibrary.MakeVector` (.x _returnvalue) (select `bool` (`self.DeckGrid?`) :`false` (`self.MinScrollDownValue`) :`true` (`self.MinScrollDownValueGrid`)) (.z _returnvalue)) (`KismetMathLibrary.MakeVector` (.x _returnvalue) (+ (.y _returnvalue) (`.DistanceBetweenFloors_7_4ECEC1AA4DF2B8434F59AABE5F8F5FCA` (break `/Game/Blueprints/Structs/s_DeckSetup` (`self.DeckListSetup`)))) (.z _returnvalue)) (<= (select `bool` (`self.DeckGrid?`) :`false` (`self.MinScrollDownValue`) :`true` (`self.MinScrollDownValueGrid`)) (.y _returnvalue))))

(fn `f_SmoothScrollUp`
  (returns (MaxScrollup :type "Vector Structure") (NextValue :type "Vector Structure") (TrueFalse :type Boolean))
  (bind _returnvalue (`self.K2_GetActorLocation` (`self.CameraRef`)))
  (bind _y (.y _returnvalue))
  (return (`KismetMathLibrary.MakeVector` (.x _returnvalue) (select `bool` (`self.DeckGrid?`) :`true` (* (`.DistanceBetweenFloors_7_4ECEC1AA4DF2B8434F59AABE5F8F5FCA` (break `/Game/Blueprints/Structs/s_DeckSetup` (`self.DeckListSetup`))) 2.0)) (.z _returnvalue)) (`KismetMathLibrary.MakeVector` (.x _returnvalue) (- _y (`.DistanceBetweenFloors_7_4ECEC1AA4DF2B8434F59AABE5F8F5FCA` (break `/Game/Blueprints/Structs/s_DeckSetup` (`self.DeckListSetup`)))) (.z _returnvalue)) (<= _y (select `bool` (`self.DeckGrid?`) :`true` (* (`.DistanceBetweenFloors_7_4ECEC1AA4DF2B8434F59AABE5F8F5FCA` (break `/Game/Blueprints/Structs/s_DeckSetup` (`self.DeckListSetup`))) 2.0)))))

(fn `GenerateGridPattern`
  (params (DecksToGenerate :type "Array of /Game/Blueprints/Ship/BP_Floor Object Reference"))
  (locals (LocalDecks :type "Array of /Game/Blueprints/Ship/BP_Floor Object Reference") (LocalModifiedDecks :type "Array of /Game/Blueprints/Ship/BP_Floor Object Reference"))
  (bind _localmodifieddecks (`local.LocalModifiedDecks`))
  (bind _gridstartpos (`self.GridStartPos`))
  (bind _gridstartpos_2 (`self.GridStartPos`))
  (bind (_returnvalue_x _returnvalue_y) (`KismetMathLibrary.BreakVector` (+ (`self.GridStartPos`) (`KismetMathLibrary.MakeVector` 0.0 (`.DistanceBetweenFloors_7_4ECEC1AA4DF2B8434F59AABE5F8F5FCA` (break `/Game/Blueprints/Structs/s_DeckSetup` (`self.DeckListSetup`)))))))
  (bind _output_get (set `local.LocalDecks` DecksToGenerate))
  (set `local.LocalModifiedDecks` _output_get)
  (if (< (`KismetArrayLibrary.Array_LastIndex` (`local.LocalDecks`)) (`self.DecksPerRow`))
    (for _array_element (`local.LocalDecks`)
      (bind _output_get_2 (set `/Game/Blueprints/Ship/BP_Floor.FloorGridLocation` _gridstartpos _array_element))
      (set `self.GridStartPos` (+ _gridstartpos (`KismetMathLibrary.MakeVector` (`.DistanceBetweenFloors_7_4ECEC1AA4DF2B8434F59AABE5F8F5FCA` (break `/Game/Blueprints/Structs/s_DeckSetup` (`self.DeckGridSetup`))))))
      (`KismetArrayLibrary.Array_Add` (`self.DeckGridPositions`) _output_get_2))
    (else
      (`KismetArrayLibrary.Array_Resize` _localmodifieddecks (`self.DecksPerRow`))
      (for _array_element_2 _localmodifieddecks
        (bind _output_get_3 (set `/Game/Blueprints/Ship/BP_Floor.FloorGridLocation` _gridstartpos_2 _array_element_2))
        (set `self.GridStartPos` (+ _gridstartpos_2 (`KismetMathLibrary.MakeVector` (`.DistanceBetweenFloors_7_4ECEC1AA4DF2B8434F59AABE5F8F5FCA` (break `/Game/Blueprints/Structs/s_DeckSetup` (`self.DeckGridSetup`))))))
        (`KismetArrayLibrary.Array_Add` (`self.DeckGridPositions`) _output_get_3))
      (set `self.GridStartPos` (`KismetMathLibrary.MakeVector` 0.0 _returnvalue_y 100.0))
      (for _array_element_3 (`local.LocalModifiedDecks`)
        (`KismetArrayLibrary.Array_RemoveItem` (`local.LocalDecks`) _array_element_3))
      (`self.GenerateGridPattern` (`local.LocalDecks`))
      (return))))

(fn `GetAlphaForTimeline`
  (params (`Timeline component` :type "TimelineComponent Object Reference"))
  (returns (Alpha :type "Float (double-precision)"))
  (return (`KismetMathLibrary.FClamp` (/ (`TimelineComponent.GetPlaybackPosition` `Timeline component`) (`TimelineComponent.GetTimelineLength` `Timeline component`)))))

(fn `GetCameraLocation`
  (returns (CameraLocation :type "Vector Structure"))
  (return (`self.K2_GetActorLocation` (`self.CameraRef`))))

(fn `GetController`
  (returns (Controller :type "/Game/Blueprints/Ruleset/ScanReach_Con Object Reference") (bSuccess :type Boolean))
  (bind (_asscan_reach_con _bsuccess) (cast `/Game/Blueprints/Ruleset/ScanReach_Con` (`GameplayStatics.GetPlayerController` 0) :!pure true))
  (return _asscan_reach_con _bsuccess))

(fn `GetDeckScale`
  (returns (DeckScale :type "Vector Structure"))
  (bind ((`DeckScale_21_88CECE8E4A64988FBC393A8AF6C8430C` _deckscale)) (break `/Game/Blueprints/Structs/s_DeckSetup` (`self.DeckListSetup`)))
  (return (`KismetMathLibrary.MakeVector` _deckscale _deckscale _deckscale)))

(fn `GetDistanceBetweenFloors`
  (returns (DistanceBetweenFloors :type "Float (double-precision)"))
  (return (`.DistanceBetweenFloors_7_4ECEC1AA4DF2B8434F59AABE5F8F5FCA` (break `/Game/Blueprints/Structs/s_DeckSetup` (`self.DeckListSetup`)))))

(fn `GetFloors`
  (returns (`Floors Array` :type "Array of /Game/Blueprints/Structs/s_FloorInfo Structure"))
  (return (`.Decks_15_4BEBB74B4BD5233113329891216757F0` (break `/Game/Blueprints/Structs/s_DeckSetup` (`self.DeckListSetup`)))))

(fn `GetNameSize`
  (returns (NameSIze :type "Float (double-precision)"))
  (return (`.NameSize_9_7556AA284F455C187F2E3E85FC87BF16` (break `/Game/Blueprints/Structs/s_DeckSetup` (`self.DeckListSetup`)))))

(fn `GetTriggerScale`
  (returns (TriggerScale :type "Vector Structure"))
  (return (`.TriggerScale_22_EF520A1244B90B5CD1394D9B2D0A12F0` (break `/Game/Blueprints/Structs/s_DeckSetup` (`self.DeckListSetup`)))))

(fn `UserConstructionScript`
  (locals (DeckStartingPos :type "Vector Structure" :default (0.0 0.0 100.0)))
  (bind _deckstartingpos (`local.DeckStartingPos`))
  (bind ((`DistanceBetweenFloors_7_4ECEC1AA4DF2B8434F59AABE5F8F5FCA` _distancebetweenfloors) (`TriggerScale_22_EF520A1244B90B5CD1394D9B2D0A12F0` _triggerscale)) (break `/Game/Blueprints/Structs/s_DeckSetup` (`self.DeckGridSetup`)))
  (bind ((`DistanceBetweenFloors_7_4ECEC1AA4DF2B8434F59AABE5F8F5FCA` _distancebetweenfloors_2) (`NameSize_9_7556AA284F455C187F2E3E85FC87BF16` _namesize) (`TriggerScale_22_EF520A1244B90B5CD1394D9B2D0A12F0` _triggerscale_2) (`DeckScale_21_88CECE8E4A64988FBC393A8AF6C8430C` _deckscale) (`NameLocation_18_07272B6744170C076B9F83B48BC6B58E` _namelocation)) (break `/Game/Blueprints/Structs/s_DeckSetup` (`self.DeckListSetup`)))
  (`KismetArrayLibrary.Array_Clear` (`self.Decks`))
  (for (_array_element _array_index) (`self.GetFloors`)
    (bind (_floorname _floorimage) (break `/Game/Blueprints/Structs/s_FloorInfo` _array_element))
    (`self.f_CreateNewDeck` _floorname _floorimage _array_index _deckstartingpos _deckscale _namesize (select `bool` (`self.DeckGrid?`) :`false` _triggerscale_2 :`true` _triggerscale) _namelocation)
    (set `local.DeckStartingPos` (select `bool` (`self.DeckGrid?`) :`false` (+ _deckstartingpos (`KismetMathLibrary.MakeVector` 0.0 _distancebetweenfloors_2)) :`true` (+ _deckstartingpos (`KismetMathLibrary.MakeVector` _distancebetweenfloors))))))