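; Zoom camera actor that follows the mouse cursor in X and Y, holding a scene capture at a configurable height.
; A looping timer started on BeginPlay replaces Tick to drive the updates.
; Each update offsets the deprojected cursor origin along its ray by origin Z over direction Z, without a trace, to position the actor.
; It also applies the OrthoWidth variable to the capture component, setting the orthographic zoom.
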(event `self.ReceiveBeginPlay`
  (`KismetSystemLibrary.K2_SetTimerDelegate` (delegate `OutsideTick`) 0.02 true))

(event `OutsideTick`
  (bind (_worldlocation _worlddirection) (`PlayerController.DeprojectMousePositionToWorld` (`GameplayStatics.GetPlayerController` 0)))
  (`self.K2_SetActorLocation` (`KismetMathLibrary.MakeVector` (.x (+ _worldlocation (* _worlddirection (/ (.z _worldlocation) (.z _worlddirection))))) (.y (+ _worldlocation (* _worlddirection (/ (.z _worldlocation) (.z _worlddirection))))) (`self.ZoomDistance`)))
  (set `SceneCaptureComponent2D.OrthoWidth` (`self.OrthoWidth`) (`self.CaptureComponent2D`)))

(fn `UserConstructionScript`)